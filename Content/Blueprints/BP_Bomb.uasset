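; BP_Bomb is a bomb pickup that penalizes the character who picks it up.
; Its PickUp Effect decreases the score through the GameMode, then applies its Damage value to the character with the DT_Bomb damage type.
; An upward impulse on the character's movement is present but disconnected, and Add Stars is empty.
; The event graph holds only disabled stub events.
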(fn `Add_Stars`)

(fn `PickUp_Effect`
  (params (GameMode :type "/Game/ThirdPerson/Blueprints/BP_ThirdPersonGameMode Object Reference") (Character :type "/Game/ThirdPerson/Blueprints/BP_Master_Character Object Reference"))
  ; Decrease Score
  (`/Game/ThirdPerson/Blueprints/BP_ThirdPersonGameMode.Decrease Score` GameMode)
  ; Apply Damage
  (`GameplayStatics.ApplyDamage` Character (`self.Damage`) null null "/Game/Blueprints/DT_Bomb.DT_Bomb_C"))

(fn `UserConstructionScript`
  (`parent.UserConstructionScript`))