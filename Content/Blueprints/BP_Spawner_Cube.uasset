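; BP_Spawner_Cube is an interactable cube spawner that creates one BP_Ball each time its Interact event fires.
; Each ball appears at a random XY offset within SpawnAreaSize of the cube, raised by the BallHeight passed into the event.
; It tracks spawned balls in an array and counter; once MaxSpawnCount is reached, the next interaction destroys them all, resets and spawns afresh.
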(event `/Game/Blueprints/I_Interactable.Interact`
  (params (BallHeight :type "Float (double-precision)"))
  (bind _spawn_area_size (`self.Spawn_Area_Size`))
  (bind _returnvalue (* _spawn_area_size -1.0))
  ; Spawn Balls On Interact
  ;; Check if Max Objects are Spawned
  (if (>= (`self.Spawned_Number`) (`self.Max_Spawn_Count`))
    ;; Reset When Max Objects Spawned
    (for _array_element (`self.Spawned_Objects`)
      (if (!= _array_element null)
        (`self.K2_DestroyActor` _array_element)))
    (set `self.Spawned_Number` 0)
    (set `self.Spawned_Objects` (`|MakeArray` null :!type "/Game/Blueprints/BP_Ball Object Reference")))
  (bind _returnvalue_2 (`|SpawnActorFromClass` "/Game/Blueprints/BP_Ball.BP_Ball_C" (`KismetMathLibrary.Conv_VectorToTransform` (+ (`SceneComponent.K2_GetComponentLocation` (`self.Cube`)) (`KismetMathLibrary.MakeVector` (`KismetMathLibrary.RandomFloatInRange` _returnvalue _spawn_area_size) (`KismetMathLibrary.RandomFloatInRange` _returnvalue _spawn_area_size) BallHeight))) "Undefined" "MultiplyWithRoot" null null))
  ;; Update Spawned Number & List
  (`KismetArrayLibrary.Array_Append` (`self.Spawned_Objects`) (`|MakeArray` _returnvalue_2))
  (`/Engine/EditorBlueprintResources/StandardMacros.IncrementInt` (`self.Spawned_Number`)))

(fn `UserConstructionScript`)