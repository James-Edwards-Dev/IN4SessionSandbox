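; BP_PickUp is a spinning collectible with a pulsing point light that adds score when collected.
; On overlap by a master character it plays a sound, calls PickUpEffect, which scores only for BP_ThirdPersonCharacter, then has the game mode respawn it.
; If Colourful, construction and pickup randomise a shared light and dynamic material colour; otherwise construction removes the light and Niagara.
; Star spawning and cleanup logic exists but is disconnected.
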(event `self.ReceiveBeginPlay`)

(event `self.ReceiveTick`
  (params (DeltaSeconds :type "Float (single-precision)"))
  (bind _pointlight (`self.PointLight`))
  (bind _returnvalue (* (`self.Light_Change_Rate`) DeltaSeconds))
  (bind _intensity (`LightComponentBase.Intensity` (`self.PointLight`)))
  (bind _intensity_2 (`LightComponentBase.Intensity` (`self.PointLight`)))
  ; Add Rotation
  (if (not (`self.bHidden`))
    (`SceneComponent.K2_AddLocalRotation` (`self.DefaultSceneRoot`) (`KismetMathLibrary.MakeRotator` 0.0 0.0 (* DeltaSeconds (`self.Rotation Speed`))) false false)
    ; Intensity Change Dirrection
    (if (`KismetSystemLibrary.IsValid` (`self.PointLight`))
      (if (>= _intensity (`self.Max_Intensity`))
        (set `self.Increase_Intensity` false)
        (elif (<= _intensity (`self.Min_Intensity`))
          (set `self.Increase_Intensity` true)))
      ; Increase/Decrease Intensity
      (if (`self.Increase_Intensity`)
        (`LightComponent.SetIntensity` _pointlight (+ _intensity_2 _returnvalue))
        (else
          (`LightComponent.SetIntensity` _pointlight (- _intensity_2 _returnvalue)))))))

(event `self.CollisionBox.OnComponentBeginOverlap`
  (params (OverlappedComponent :type "PrimitiveComponent Object Reference") (OtherActor :type "Actor Object Reference") (OtherComp :type "PrimitiveComponent Object Reference") (OtherBodyIndex :type Integer) (bFromSweep :type Boolean) (SweepResult :type "HitResult Structure (by ref)"))
  ; Collision With Trigger
  (bind _asbp_master_character (cast `/Game/ThirdPerson/Blueprints/BP_Master_Character` OtherActor))
  (`GameplayStatics.PlaySoundAtLocation` (`AudioComponent.Sound` (`self.Audio`)) (`SceneComponent.K2_GetComponentLocation` (`self.DefaultSceneRoot`)) (struct) 1.0 1.0 0.0 null null null null)
  (bind _asbp_third_person_game_mode (cast `/Game/ThirdPerson/Blueprints/BP_ThirdPersonGameMode` (`GameplayStatics.GetGameMode`)))
  (`self.PickUp_Effect` _asbp_third_person_game_mode _asbp_master_character)
  (`/Game/ThirdPerson/Blueprints/BP_ThirdPersonGameMode.Respawn_PickUp` _asbp_third_person_game_mode self (`SceneComponent.K2_GetComponentToWorld` (`self.DefaultSceneRoot`)))
  (`self.Randomise Light and Material Colour`))

(fn `Add_Stars`
  (for _ (range 3)
    (bind _returnvalue (`|SpawnActorFromClass` "/Game/Blueprints/BP_Start_Actor.BP_Start_Actor_C" (`KismetMathLibrary.MakeTransform` (+ (`KismetMathLibrary.MakeVector` (`KismetMathLibrary.RandomFloatInRange` -50.0 50.0) (`KismetMathLibrary.RandomFloatInRange` -50.0 50.0) (`KismetMathLibrary.RandomFloatInRange` -50.0 50.0)) (.location (`SceneComponent.K2_GetComponentToWorld` (`self.DefaultSceneRoot`)))) (.rotation (`SceneComponent.K2_GetComponentToWorld` (`self.DefaultSceneRoot`))) (.scale (`SceneComponent.K2_GetComponentToWorld` (`self.DefaultSceneRoot`)))) "Undefined" "MultiplyWithRoot" null null))
    (`KismetArrayLibrary.Array_Append` (`self.Star_Array`) (`|MakeArray` _returnvalue))
    (`PrimitiveComponent.SetMaterial` (`/Game/Blueprints/BP_Start_Actor.StaticMesh` _returnvalue) 0 (`self.Dynamic_Material`))))

(fn `PickUp_Effect`
  (params (GameMode :type "/Game/ThirdPerson/Blueprints/BP_ThirdPersonGameMode Object Reference") (Character :type "/Game/ThirdPerson/Blueprints/BP_Master_Character Object Reference"))
  (cast `/Game/ThirdPerson/Blueprints/BP_ThirdPersonCharacter` Character)
  (`/Game/ThirdPerson/Blueprints/BP_ThirdPersonGameMode.Increase Score` GameMode))

(fn `Randomise Light and Material Colour`
  (if (`self.bColourful`)
    ; Color
    (set `self.Linear Color` (make `LinearColor` (`KismetMathLibrary.RandomFloat`) (`KismetMathLibrary.RandomFloat`) (`KismetMathLibrary.RandomFloat`) 1.0))
    ; Material
    (bind _returnvalue (`KismetMaterialLibrary.CreateDynamicMaterialInstance` (`self.Material`)))
    (bind _output_get (set `self.Dynamic_Material` _returnvalue))
    (`MaterialInstanceDynamic.SetVectorParameterValue` _output_get "Color_Variable" (`self.Linear Color`))
    (`PrimitiveComponent.SetMaterial` (`self.StaticMesh`) 0 (`self.Dynamic_Material`))
    ; Light
    (`LightComponent.SetLightColor` (`self.PointLight`) (`self.Linear Color`) true)))

(fn `UserConstructionScript`
  (if (`self.bColourful`)
    (`self.Randomise Light and Material Colour`)
    (else
      (`ActorComponent.K2_DestroyComponent` (`self.PointLight`))
      (`ActorComponent.K2_DestroyComponent` (`self.Niagara`))))
  ; Set Scale
  (`SceneComponent.SetWorldScale3D` (`self.StaticMesh`) (`self.Scale`))
  ; Set Rotation
  (`SceneComponent.K2_SetWorldRotation` (`self.StaticMesh`) (`self.Rotation`) false false))