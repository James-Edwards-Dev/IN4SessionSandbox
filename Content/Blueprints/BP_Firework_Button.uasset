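; BP_Firework_Button is an interactable button that fires a colored firework through CallFirework when Interact is triggered.
; Its construction script randomizes the color that is passed with that call.
; A sphere overlap shows and hides an "E / Interact" tooltip widget for BP_ThirdPersonCharacter.
; Tick rotates the tooltip to face the player camera.
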(event `self.ReceiveTick`
  (params (DeltaSeconds :type "Float (single-precision)"))
  (`SceneComponent.K2_SetWorldRotation` (`self.Tooltip`) (`KismetMathLibrary.FindLookAtRotation` (`SceneComponent.K2_GetComponentLocation` (`self.Tooltip`)) (`SceneComponent.K2_GetComponentLocation` (`PlayerCameraManager.TransformComponent` (`GameplayStatics.GetPlayerCameraManager` 0)))) false false))

(event `self.ReceiveBeginPlay`
  ; Update Tool Tip
  (bind _asbpw_tool_tip (cast `/Game/UI/BPW_Tool_Tip` (`WidgetComponent.GetWidget` (`self.Tooltip`))))
  (set `/Game/UI/BPW_Tool_Tip.Input` "E" _asbpw_tool_tip)
  (set `/Game/UI/BPW_Tool_Tip.Action` "Interact" _asbpw_tool_tip))

(event `/Game/Blueprints/I_Interactable.Interact`
  (params (BallHeight :type "Float (double-precision)"))
  (`self.Firework` (`self.Color`)))

(event `self.Sphere.OnComponentBeginOverlap`
  (params (OverlappedComponent :type "PrimitiveComponent Object Reference") (OtherActor :type "Actor Object Reference") (OtherComp :type "PrimitiveComponent Object Reference") (OtherBodyIndex :type Integer) (bFromSweep :type Boolean) (SweepResult :type "HitResult Structure (by ref)"))
  (if (== (`GameplayStatics.GetObjectClass` OtherActor) "/Game/ThirdPerson/Blueprints/BP_ThirdPersonCharacter.BP_ThirdPersonCharacter_C")
    (`SceneComponent.SetHiddenInGame` (`self.Tooltip`) false false)))

(event `self.Sphere.OnComponentEndOverlap`
  (params (OverlappedComponent :type "PrimitiveComponent Object Reference") (OtherActor :type "Actor Object Reference") (OtherComp :type "PrimitiveComponent Object Reference") (OtherBodyIndex :type Integer))
  (if (== (`GameplayStatics.GetObjectClass` OtherActor) "/Game/ThirdPerson/Blueprints/BP_ThirdPersonCharacter.BP_ThirdPersonCharacter_C")
    (`SceneComponent.SetHiddenInGame` (`self.Tooltip`) true false)))

(fn `UserConstructionScript`
  ; Randomise Effect Colour
  (set `self.Color` (`KismetMathLibrary.MakeColor` (`KismetMathLibrary.RandomFloat`) (`KismetMathLibrary.RandomFloat`) (`KismetMathLibrary.RandomFloat`))))